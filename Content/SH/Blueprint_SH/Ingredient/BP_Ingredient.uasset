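; BP_Ingredient is a food ingredient actor that changes its mesh as it touches kitchen objects.
; On BeginPlay it loads its row from DT_Ingredient by RowName, stores it, spawns an emitter and shows the uncooked mesh.
; Overlaps on the mesh component cast the other actor: BP_CuttingBoard swaps in the cooked mesh, BP_Plate the food mesh, with no check on the current stage.
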(event `self.ReceiveBeginPlay`
  (bind _returnvalue (`|GetDataTableRow` "/Game/SH/DT_SH/DT_Ingredient.DT_Ingredient" (`self.Row Name`))
    (:`then`
      (bind _output_get (set `self.St_Uncooked` _returnvalue))
      (`GameplayStatics.SpawnEmitterAtLocation` null)
      (`StaticMeshComponent.SetStaticMesh` (`self.Ingredient`) (`.UncookedST_22_C29EBA134FBDAC2FF85EF4B432329BF6` (break `/Game/SH/DT_SH/ST_Ingredient` _output_get))))))

(event `self.Ingredient.OnComponentBeginOverlap`
  (params (OverlappedComponent :type "PrimitiveComponent Object Reference") (OtherActor :type "Actor Object Reference") (OtherComp :type "PrimitiveComponent Object Reference") (OtherBodyIndex :type Integer) (bFromSweep :type Boolean) (SweepResult :type "HitResult Structure (by ref)"))
  (`self.OverlapCuttingBoard` OtherActor)
  (`self.OverlapPlate` OtherActor))

(fn `OverlapCuttingBoard`
  (params (Object :type "Object Object Reference"))
  (cast `/Game/SH/Blueprint_SH/Tools/BP_CuttingBoard` Object)
  (`StaticMeshComponent.SetStaticMesh` (`self.Ingredient`) (`.CookedST_23_29685B244667E89A05184CA44BA7BE77` (break `/Game/SH/DT_SH/ST_Ingredient` (`self.St_Uncooked`)))))

(fn `OverlapPlate`
  (params (Object :type "Object Object Reference"))
  (cast `/Game/SH/Blueprint_SH/Food/BP_Plate` Object)
  (`StaticMeshComponent.SetStaticMesh` (`self.Ingredient`) (`.FoodST_25_B739C11D477948B342A07B8756BC99D5` (break `/Game/SH/DT_SH/ST_Ingredient` (`self.St_Uncooked`)))))

(fn `UserConstructionScript`)